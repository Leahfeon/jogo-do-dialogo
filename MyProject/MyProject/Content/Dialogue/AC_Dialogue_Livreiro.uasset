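; Dialogue component for Owen, the Livraria Santiago bookseller, who greets journalist Aria and points her to a book about the Óbidos rumor.
; Its Dialogue function calls the parent, then chains single-option AddDialogue exchanges through their Pass Through state.
; The last exchange clears dialogue progress and closes the conversation.
; Three short exchanges with Portuguese text remain unconnected and never run.
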(fn `Dialogue`
  (`parent.Dialogue`)
  (switch `int` (`self.DialogueTreeIndex`)
    (:`Default`
      (bind _state (`self.AddDialogue` "Bookseller" "(With a friendly smile) Welcome to Livraria Santiago. I'm Owen, the bookseller here." (`|MakeArray` " (with enthusiasm) Hi, Owen! I'm Aria." :!type "Text")))
      (switch `/Game/Dialogue/Enum_DialogueState` _state
        (:`NewEnumerator0`
          (bind _state_2 (`self.AddDialogue` "Owen" "(nodding) Pleasure to meet you, Aria. You seem to be new around here. What brings you to Livraria Santiago?" (`|MakeArray` "(looking around) Well, I'm a journalist from The Outside. It's a place where physical books are becoming rare. There's this rumor about Óbidos, and I heard this bookstore might have answers." :!type "Text")))
          (switch `/Game/Dialogue/Enum_DialogueState` _state_2
            (:`NewEnumerator0`
              (bind _state_3 (`self.AddDialogue` "Owen" "The Outside, huh? That's quite a distance. (smiling) Well, you've come to the right place. Livraria Santiago holds stories from every corner of the world." (`|MakeArray` "That's amazing! People out there don't realize how important physical books are. They're like portals to different worlds." :!type "Text")))
              (switch `/Game/Dialogue/Enum_DialogueState` _state_3
                (:`NewEnumerator0`
                  (bind _state_4 (`self.AddDialogue` "Owen" " I couldn't agree more, Aria. Books have a unique magic that e-books just can't capture. So, about this rumor regarding Óbidos, are you here to investigate?" (`|MakeArray` "Absolutely! I believe in the power of books, and if there's something happening in Óbidos that's connected to them, I want to know." :!type "Text")))
                  (switch `/Game/Dialogue/Enum_DialogueState` _state_4
                    (:`NewEnumerator0`
                      (bind _state_5 (`self.AddDialogue` "Owen" "Well then, Aria, you're in for a treat. Near that stained glass over there is a book I think you might find intriguing. It holds a tale that might shed some light on your quest." (`|MakeArray` "Really? I can't wait to read it! What's the book called?" :!type "Text")))
                      (switch `/Game/Dialogue/Enum_DialogueState` _state_5
                        (:`NewEnumerator0`
                          (`self.ClearDialogueProgress`)
                          (`self.CloseConversation`))))))))))))))