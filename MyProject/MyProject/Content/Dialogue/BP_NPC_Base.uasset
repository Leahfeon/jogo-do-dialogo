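; Base NPC Blueprint for the dialogue system, with a name label that signals when the character can be interacted with.
; The construction script writes CharacterName into the TxtCharacterName component, and SetInteractableState shows or hides that label.
; When ConversationClosed fires, it forwards a ConversationClosedMessage to the stored InteractInstigator.
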(event `/Game/Dialogue/BPI_Interactable.SetInteractableState`
  (params (`bCanShowInteract?` :type Boolean))
  (if `bCanShowInteract?`
    (`SceneComponent.SetVisibility` (`self.txt_CharacterName`) true false)
    (else
      (`SceneComponent.SetVisibility` (`self.txt_CharacterName`) false false))))

(event `/Game/Dialogue/BPI_Interactable.ConversationClosed`
  (message `/Game/Dialogue/BPI_Interactable.ConversationClosed` (`self.InteractInstigator`)))

(fn `UserConstructionScript`
  (`TextRenderComponent.K2_SetText` (`self.txt_CharacterName`) (`self.CharacterName`)))